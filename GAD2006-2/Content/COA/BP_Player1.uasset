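; BP_Player1 is a player Blueprint that shows a stamina UI and debug readouts of its stamina state.
; BeginPlay creates the WB_Stamina widget and adds it to the viewport.
; Tick prints StaminaGainDelay and CurrentStamina on screen every frame, but no graph here changes either value.
; ModifyDamage returns incoming damage unchanged, and the construction script is empty.
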(event `self.ReceiveBeginPlay`
  (bind _returnvalue (`|CreateWidget` "/Game/COA/WB_Stamina.WB_Stamina_C"))
  (`UserWidget.AddToViewport` _returnvalue 0))

(event `self.ReceiveTick`
  (params (DeltaSeconds :type "Float (single-precision)"))
  (`KismetSystemLibrary.PrintString` (`KismetStringLibrary.Concat_StrStr` "Stamina Gain Delay: " (`KismetStringLibrary.Conv_DoubleToString` (`self.StaminaGainDelay`))) true true (struct :`G` 0.66 :`B` 1.0 :`A` 1.0) 0.0)
  (`KismetSystemLibrary.PrintString` (`KismetStringLibrary.Concat_StrStr` "Current Stamina" (`KismetStringLibrary.Conv_DoubleToString` (`self.CurrentStamina`))) true true (struct :`R` 1.0 :`G` 0.032916 :`A` 1.0) 0.0))

(fn `ModifyDamage`
  (params (IncomingDamage :type "Float (single-precision)"))
  (returns (ReturnValue :type "Float (single-precision)"))
  (return IncomingDamage))

(fn `UserConstructionScript`)